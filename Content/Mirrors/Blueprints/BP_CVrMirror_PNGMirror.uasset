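; Mirror Blueprint that shows media on its material while the player stands inside its collision box.
; Begin overlap by player pawn 0 opens PNGMediaSource on the DesertVideo media player and raises the dynamic material's VideoAmount parameter to partially blend in the video.
; End overlap resets that parameter to zero without closing or pausing the player.
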(event `self.CollisionBox.OnComponentBeginOverlap`
  (params (OverlappedComponent :type "PrimitiveComponent Object Reference") (OtherActor :type "Actor Object Reference") (OtherComp :type "PrimitiveComponent Object Reference") (OtherBodyIndex :type Integer) (bFromSweep :type Boolean) (SweepResult :type "HitResult Structure (by ref)"))
  (if (== OtherActor (`GameplayStatics.GetPlayerPawn` 0))
    (`MediaPlayer.OpenSource` (`self.DesertVideo`) "/Game/PNGS/PNGMediaSource.PNGMediaSource")
    (`MaterialInstanceDynamic.SetScalarParameterValue` (`self.MaterialInstanceDynamic`) "VideoAmount" 0.7)))

(event `self.CollisionBox.OnComponentEndOverlap`
  (params (OverlappedComponent :type "PrimitiveComponent Object Reference") (OtherActor :type "Actor Object Reference") (OtherComp :type "PrimitiveComponent Object Reference") (OtherBodyIndex :type Integer))
  (if (== OtherActor (`GameplayStatics.GetPlayerPawn` 0))
    (`MaterialInstanceDynamic.SetScalarParameterValue` (`self.MaterialInstanceDynamic`) "VideoAmount" 0.0)))

(fn `UserConstructionScript`)